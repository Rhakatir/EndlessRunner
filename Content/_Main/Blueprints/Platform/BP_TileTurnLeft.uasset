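; Left-turn platform tile Blueprint for a runner game that controls when the RunCharacter may turn.
; Entering its CanTurnBox trigger sets CanTurn on the character and disables lane switching.
; Leaving the trigger re-enables lane switching but leaves CanTurn unchanged.
; The construction script only calls its parent, and BeginPlay is disabled.
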(event OnComponentBeginOverlap(CanTurnBox)
  (params (OverlappedComponent :type Primitive%20Component%20Object%20Reference) (OtherActor :type Actor%20Object%20Reference) (OtherComp :type Primitive%20Component%20Object%20Reference) (OtherBodyIndex :type Integer) (bFromSweep :type Boolean) (SweepResult :type Hit%20Result%20Structure%20%28by%20ref%29))
  ;[0 0 0 0.5] Set Variables
  (if (== OtherActor (Variables|Default|GetRunCharacter))
    (Variables|/Game/_Main/Blueprints/RunCharacter/RunCharacter.RunCharacter_C|SetCanTurn? (Variables|Default|GetRunCharacter) true)
    (Variables|/Game/_Main/Blueprints/RunCharacter/RunCharacter.RunCharacter_C|SetCanSwitchLane? (Variables|Default|GetRunCharacter) false)))

(event OnComponentEndOverlap(CanTurnBox)
  (params (OverlappedComponent :type Primitive%20Component%20Object%20Reference) (OtherActor :type Actor%20Object%20Reference) (OtherComp :type Primitive%20Component%20Object%20Reference) (OtherBodyIndex :type Integer))
  ;[0 0 0 0.5] Set Variables
  (if (== OtherActor (Variables|Default|GetRunCharacter))
    (Variables|/Game/_Main/Blueprints/RunCharacter/RunCharacter.RunCharacter_C|SetCanSwitchLane? (Variables|Default|GetRunCharacter) true)))

(event EventBeginPlay
  (|CallParentFunction) ; This node is disabled and will not be called.\nDrag off pins to build functionality.
)

(fn ConstructionScript
  (|CallParentFunction))